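; BP_Flower is an actor Blueprint that pulses the brightness of its PointLight over time.
; Tick accumulates delta time into a timer and takes its sine as a wave.
; That wave is averaged with a clamped copy of itself, compressing its lower portion, then scaled to set light intensity, which dips below zero at the troughs.
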(event `self.ReceiveTick`
  (params (DeltaSeconds :type "Float (single-precision)"))
  (bind _output_get (set `self.Timer` (+ (`self.Timer`) DeltaSeconds)))
  (bind _output_get_2 (set `self.LightIntensity` (`KismetMathLibrary.Sin` _output_get)))
  (`LightComponent.SetIntensity` (`self.PointLight`) (* (* (+ _output_get_2 (`KismetMathLibrary.FClamp` _output_get_2 0.7)) 0.5) 100.0)))

(fn `UserConstructionScript`)