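; Secondary crop flower actor that the third-person character can take while overlapping it, marked by a pulsing point light.
; Begin and end overlap toggle the character's CanTakeCrops flag, and both set WhichSecCrops to this actor, so the reference is not cleared on exit.
; Tick drives the light intensity from a sine of accumulated time, averaged with a clamped copy of itself to skew the pulse upward.
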(event `self.ReceiveActorEndOverlap`
  (params (OtherActor :type "Actor Object Reference"))
  (bind _asthird_person_character (cast `/Game/ThirdPersonBP/Blueprints/ThirdPersonCharacter` OtherActor))
  (set `/Game/ThirdPersonBP/Blueprints/ThirdPersonCharacter.CanTakeCrops` false _asthird_person_character)
  (set `/Game/ThirdPersonBP/Blueprints/ThirdPersonCharacter.WhichSecCrops` self _asthird_person_character))

(event `self.ReceiveActorBeginOverlap`
  (params (OtherActor :type "Actor Object Reference"))
  (bind _asthird_person_character (cast `/Game/ThirdPersonBP/Blueprints/ThirdPersonCharacter` OtherActor))
  (set `/Game/ThirdPersonBP/Blueprints/ThirdPersonCharacter.CanTakeCrops` true _asthird_person_character)
  (set `/Game/ThirdPersonBP/Blueprints/ThirdPersonCharacter.WhichSecCrops` self _asthird_person_character))

(event `self.ReceiveTick`
  (params (DeltaSeconds :type "Float (single-precision)"))
  (bind _output_get (set `self.Timer` (+ (`self.Timer`) DeltaSeconds)))
  (bind _output_get_2 (set `self.LightIntensity` (`KismetMathLibrary.Sin` _output_get)))
  (`LightComponent.SetIntensity` (`self.PointLight`) (* (* (+ _output_get_2 (`KismetMathLibrary.FClamp` _output_get_2 0.7)) 0.5) 100.0)))

(fn `UserConstructionScript`)